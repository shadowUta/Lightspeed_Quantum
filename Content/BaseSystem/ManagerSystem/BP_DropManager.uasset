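; BP_DropManager is a manager that places item drops in the world through an object pool of BP_Drop actors.
; GenerateDropItem gets a drop from FoundValidDrop, clears its validity, moves it to the given transform and repositions its Sphere, printing an error if the move fails.
; FoundValidDrop scans DropPool for a valid, available actor to reassign ItemID and Quantity, otherwise spawning one far off-position and adding it to the pool.
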(event Custom|GenerateDropItem
  (params (ItemID :type Name) (Quantity :type Integer) (Transform :type Transform))
  (bind _returndrop (CallFunction|FoundValidDrop ItemID Quantity))
  (Default|SetValidity _returndrop false)
  (bind _returnvalue (Transformation|SetActorTransform _returndrop Transform))
  (if _returnvalue
    (Transformation|SetRelativeLocation (Variables|/Game/Interactable/BP_Drop.BP_Drop_C|GetSphere _returndrop) (Transformation|GetActorLocation _returndrop) false false)
    (else
      (Development|PrintString "掉落错误"))))

(fn ConstructionScript)

(fn FoundValidDrop
  (params (ItemID :type Name) (Quantity :type Integer))
  (bind _droppool (Variables|Default|GetDropPool))
  (bind _index (LocalVariables|GetIndex))
  (bind _output (Utilities|Array|Get(acopy) _droppool _index))
  (Utilities|FlowControl|Sequence
    (:then_0
      (if (> (Utilities|Array|Length (Variables|Default|GetDropPool)) (LocalVariables|GetIndex)) :!label _label
        (if (and (Variables|/Game/Interactable/BP_Drop.BP_Drop_C|GetValidity _output) (Utilities|IsValid _output))
          (bind _output_get (LocalVariables|SetReturnActor _output))
          (Variables|/Game/Interactable/BP_Drop.BP_Drop_C|SetItem%20ID _output_get ItemID)
          (Variables|/Game/Interactable/BP_Drop.BP_Drop_C|SetQuantity _output_get Quantity)
          (else
            (Math|Integer|IncrementInt (LocalVariables|GetIndex)
              (:%20%20
                (goto _label)))))
        (else
          (bind _returnvalue (Game|SpawnActorfromClass "/Game/Interactable/BP_Drop.BP_Drop_C" (Math|Transform|MakeTransform "10000.000000,10000.000000,-10000.000000" "0, 0, 0" "1.000000,1.000000,1.000000") "AlwaysSpawn" "MultiplyWithRoot" 0 ItemID Quantity 0))
          (bind _output_get_2 (LocalVariables|SetReturnActor _returnvalue))
          (Utilities|Array|Add (Variables|Default|GetDropPool) _output_get_2))))
    (:then_1
      (return (LocalVariables|GetReturnActor)))))