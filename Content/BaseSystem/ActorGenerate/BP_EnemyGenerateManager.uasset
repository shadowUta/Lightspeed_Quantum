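; Manager actor that keeps enemies spawning around the player, up to a maximum count.
; On BeginPlay it async-loads a generate data asset for the class list, then starts two looping timers.
; GenerateTimer spawns a random class at a navmesh-projected random offset from the player, and stops its timer if the list is empty.
; ClearArray prunes invalid actors from the tracked array that the cap checks.
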(event Custom|GenerateTimer
  (bind _returnvalue (Game|Player|GetPlayerPawn 0))
  (bind _returnvalue_2 (Math|Random|RandomFloatinRange -1.8e+02 1.8e+02))
  (bind _maxrange (Variables|Default|GetMaxRange))
  (bind _minrange (Variables|Default|GetMinRange))
  (bind _returnvalue_3 (Transformation|GetActorLocation _returnvalue))
  (bind _returnvalue_4 (Math|Random|RandomFloatinRange _minrange _maxrange))
  (bind _returnvalue_5 (Math|Trig|Cos(Degrees) _returnvalue_2))
  (bind _returnvalue_6 (Math|Trig|Sin(Degrees) _returnvalue_2))
  (bind _returnvalue_7 (* _returnvalue_4 _returnvalue_6))
  (bind _returnvalue_8 (* _returnvalue_4 _returnvalue_5))
  (bind _returnvalue_9 (Math|Vector|MakeVector _returnvalue_8 _returnvalue_7 0.0))
  (bind _returnvalue_10 (+ _returnvalue_3 _returnvalue_9))
  (bind (_projectedlocation _returnvalue_11) (AI|Navigation|ProjectPointtoNavigation _returnvalue_10 0 0 "0, 0, 0"))
  (if (Utilities|Array|IsNotEmpty (Variables|Default|GetActor%20Class%20Data%20Array))
    (if (< (Utilities|Array|Length (Variables|Default|GetActorArray)) (Variables|Default|GetMaxEnemyCount))
      (if _returnvalue_11
        (bind _returnvalue_12 (Game|SpawnActorfromClass (.OutItem (Utilities|Array|Random (Variables|Default|GetActor%20Class%20Data%20Array))) (Math|Transform|MakeTransform (+ _projectedlocation "0.000000,0.000000,100.000000") "0, 0, 0" "1.000000,1.000000,1.000000") "AdjustIfPossibleButDontSpawnIfColliding" "MultiplyWithRoot" 0 0))
        (Utilities|Array|Add (Variables|Default|GetActorArray) _returnvalue_12)))
    (else
      (Utilities|Time|ClearandInvalidateTimerbyHandle (Variables|Default|GetTimer)))))

(event EventBeginPlay
  (bind _object (Utilities|AsyncLoadAsset (Variables|Default|GetAsset))
    (:Completed
      (bind _aspda_generate_data (Utilities|Casting|CastToPDA_GenerateData _object))
      (Variables|Default|SetActor%20Class%20Data%20Array (Default|GetGenerateData _aspda_generate_data))
      (bind _returnvalue (Utilities|Time|SetTimerbyEvent (EventDispatchers|CreateEvent :!event Custom|GenerateTimer) 0.05 true))
      (Variables|Default|SetTimer _returnvalue)
      (Utilities|Time|SetTimerbyEvent (EventDispatchers|CreateEvent :!event ClearArray) 1.0 true))))

(fn ConstructionScript)

(fn ClearArray
  (for _array_element (Variables|Default|GetActorArray)
    (Utilities|IsValid _array_element
      (:Is%20Not%20Valid
        (Utilities|Array|Add (LocalVariables|GetArray) _array_element))))
  (for _array_element_2 (LocalVariables|GetArray)
    (Utilities|Array|RemoveItem (Variables|Default|GetActorArray) _array_element_2)))