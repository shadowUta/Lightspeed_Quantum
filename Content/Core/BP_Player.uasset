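; Player character Blueprint that routes Enhanced Input movement, interaction and inventory, with Space firing a test ability assigned to slot 0.
; Overlaps on InteractionCollision gather actors with active InteractableComponents and pass them to the InteractionComponent.
; Each tick, a camera-to-capsule sphere trace sets a "Switch" material parameter on occluding static meshes, resetting those from the previous frame that no longer block.
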(event OnComponentBeginOverlap(InteractionCollision)
  (params (OverlappedComponent :type Primitive%20Component%20Object%20Reference) (OtherActor :type Actor%20Object%20Reference) (OtherComp :type Primitive%20Component%20Object%20Reference) (OtherBodyIndex :type Integer) (bFromSweep :type Boolean) (SweepResult :type Hit%20Result%20Structure%20%28by%20ref%29))
  (if (Actor|ActorHasTag OtherActor "Interactable")
    (bind _interactable_actors (CallFunction|UpdateInteractableActor (Collision|GetOverlappingActors (Variables|Default|GetInteractionCollision) 0 :!class /Script/Engine.PrimitiveComponent)))
    (Default|UpdateList (Variables|Default|GetInteractionComponent) _interactable_actors)))

(event OnComponentEndOverlap(InteractionCollision)
  (params (OverlappedComponent :type Primitive%20Component%20Object%20Reference) (OtherActor :type Actor%20Object%20Reference) (OtherComp :type Primitive%20Component%20Object%20Reference) (OtherBodyIndex :type Integer))
  (if (Actor|ActorHasTag OtherActor "Interactable")
    (bind _interactable_actors (CallFunction|UpdateInteractableActor (Collision|GetOverlappingActors (Variables|Default|GetInteractionCollision) 0 :!class /Script/Engine.PrimitiveComponent)))
    (Default|UpdateList (Variables|Default|GetInteractionComponent) _interactable_actors)))

(event Input|EnhancedActionEvents|EnhancedInputActionIA_E
  (params (ActionValue :type Boolean) (ElapsedSeconds :type Float%20%28double-precision%29) (TriggeredSeconds :type Float%20%28double-precision%29) (InputAction :type Input%20Action%20Object%20Reference :default "/Game/Core/Input/IA_E.IA_E"))
  (:Started
    (Default|TriggerInteraction (Variables|Default|GetInteractionComponent))))

(event Input|EnhancedActionEvents|EnhancedInputActionIA_Move
  (params (ActionValue :type Vector%202D%20Structure) (ElapsedSeconds :type Float%20%28double-precision%29) (TriggeredSeconds :type Float%20%28double-precision%29) (InputAction :type Input%20Action%20Object%20Reference :default "/Game/Core/Input/IA_Move.IA_Move"))
  (Pawn|Input|AddMovementInput (Math|Vector|MakeVector (.x ActionValue) (.y ActionValue) 0.0) 1.0 false))

(event Input|EnhancedActionEvents|EnhancedInputActionIA_B
  (params (ActionValue :type Boolean) (ElapsedSeconds :type Float%20%28double-precision%29) (TriggeredSeconds :type Float%20%28double-precision%29) (InputAction :type Input%20Action%20Object%20Reference :default "/Game/Core/Input/IA_B.IA_B"))
  (:Started
    (Class|InventoryComponent|OpenInventory (Variables|Default|GetInvertoryComponent))))

(event EventBeginPlay
  (Input|AddMappingContext (PlayerController|LocalPlayerSubsystems|GetEnhancedInputLocalPlayerSubsystem (Game|GetPlayerController 0)) "/Game/Core/Input/IMC_Default.IMC_Default" 0 "(bIgnoreAllPressedKeysUntilRelease=True,bForceImmediately=False,bNotifyUserSettings=False)")
  (Default|ReplaceAbility (Variables|Default|GetAbilityComponent) 0 "(TagName=\"Ability.Test\")"))

(event EventTick
  (params (DeltaSeconds :type Float%20%28single-precision%29))
  (CallFunction|OcclusionBlur))

(event Input|KeyboardEvents|SpaceBar
  (params (Key :type Key%20Structure :default "None"))
  (bind _abilitycomponent (Variables|Default|GetAbilityComponent))
  (:Pressed
    (Utilities|IsValid _abilitycomponent
      (:Is%20Valid
        (Default|ActivateAbility _abilitycomponent)))))

(fn ConstructionScript
  (|CallParentFunction))

(fn OcclusionBlur
  (bind _temp (Variables|遮挡虚化|GetTemp))
  (bind _outhits (Collision|MultiSphereTraceForObjects (Transformation|GetWorldLocation (Variables|Default|GetCamera)) (Transformation|GetWorldLocation (Variables|Default|GetCapsuleComponent)) 5e+01 (Utilities|Array|MakeArray "ObjectTypeQuery1") false 0 "None"))
  (for _array_element _outhits
    (bind _as静态网格体actor (Utilities|Casting|CastToStaticMeshActor (.HitActor (Collision|BreakHitResult _array_element))))
    (Utilities|Set|Add (Variables|遮挡虚化|GetTemp) _as静态网格体actor)
    (bind _returnvalue (Rendering|Material|CreateDynamicMaterialInstance (Variables|/Script/Engine.StaticMeshActor|GetStaticMeshComponent _as静态网格体actor) 0 (Rendering|Material|GetMaterial (Variables|/Script/Engine.StaticMeshActor|GetStaticMeshComponent _as静态网格体actor) 0) "None" :!class /Script/Engine.PrimitiveComponent))
    (Rendering|Material|SetScalarParameterValue _returnvalue "Switch" 1.0 :!class /Script/Engine.MaterialInstanceDynamic))
  (bind _result (Utilities|Set|ToArray (Variables|遮挡虚化|GetLastMesh)))
  (for _array_element_2 _result
    (if (not (Utilities|Set|Contains (Variables|遮挡虚化|GetTemp) _array_element_2))
      (bind _returnvalue_2 (Rendering|Material|CreateDynamicMaterialInstance (Variables|/Script/Engine.StaticMeshActor|GetStaticMeshComponent _array_element_2) 0 (Rendering|Material|GetMaterial (Variables|/Script/Engine.StaticMeshActor|GetStaticMeshComponent _array_element_2) 0) "None" :!class /Script/Engine.PrimitiveComponent))
      (Rendering|Material|SetScalarParameterValue _returnvalue_2 "Switch" 0.0 :!class /Script/Engine.MaterialInstanceDynamic)))
  (Variables|遮挡虚化|SetLastMesh _temp)
  (Utilities|Set|Clear _temp))

(fn UpdateInteractableActor
  (params (Others :type Array%20of%20Actor%20Object%20References))
  (for _array_element Others
    (Utilities|IsValid (Actor|GetComponentbyClass _array_element "/Game/BaseSystem/InteractionSystem/InteractableComponent.InteractableComponent_C")
      (:Is%20Valid
        (if (Variables|/Game/BaseSystem/InteractionSystem/InteractableComponent.InteractableComponent_C|GetInteractable (Actor|GetComponentbyClass _array_element "/Game/BaseSystem/InteractionSystem/InteractableComponent.InteractableComponent_C"))
          (Utilities|Array|Add (LocalVariables|GetInteractableActors) _array_element)))))
  (return (LocalVariables|GetInteractableActors)))