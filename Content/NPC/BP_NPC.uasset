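; BP_NPC is an interactable NPC that starts a dialogue when the player triggers it.
; Its InteractableComponent trigger is gated by the Lock and Interactable flags, and Once clears Lock so the interaction fires only one time.
; TriggerEvent disables interaction and passes a hard-coded dialogue ID to DialogueComponent, whose DialogueCompleted event makes the NPC interactable again.
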(event TriggerInteraction(InteractableComponent)
  (if (Variables|Default|GetLock)
    (if (Variables|/Game/BaseSystem/InteractionSystem/InteractableComponent.InteractableComponent_C|GetInteractable (Variables|Default|GetInteractableComponent))
      (if (Variables|Default|GetOnce)
        (Variables|Default|SetLock false))
      (CallFunction|TriggerEvent))))

(event DialogueCompleted(DialogueComponent)
  (Variables|/Game/BaseSystem/InteractionSystem/InteractableComponent.InteractableComponent_C|SetInteractable (Variables|Default|GetInteractableComponent) true))

(event Custom|TriggerEvent
  (Variables|/Game/BaseSystem/InteractionSystem/InteractableComponent.InteractableComponent_C|SetInteractable (Variables|Default|GetInteractableComponent) false)
  (Default|ActivateDialogue (Variables|Default|GetDialogueComponent) (Utilities|Array|MakeArray "1001")))

(event EventBeginPlay)

(event Collision|EventActorBeginOverlap
  (params (OtherActor :type Actor%20Object%20Reference)))

(event EventTick
  (params (DeltaSeconds :type Float%20%28single-precision%29)))

(fn ConstructionScript)