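; BP_Drop is an interactable dropped item holding an ItemID and Quantity that can be picked up into an inventory.
; Interaction passes both to the instigator's BP_InventoryComponent, then destroys the actor or keeps the leftover quantity.
; That leftover check runs even when no inventory is found.
; GetInteractionData looks up name and icon in the player pawn's item DataTable, falling back to a question-mark icon.
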(event TriggerInteraction(InteractableComponent)
  (params (Instigator :type Actor%20Object%20Reference))
  (CallFunction|AddtoInventory Instigator))

(fn ConstructionScript
  (|CallParentFunction))

(fn AddtoInventory
  (params (Instigator :type Actor%20Object%20Reference))
  (bind _returnvalue (Actor|GetComponentbyClass Instigator "/Inventory/BP_InventoryComponent.BP_InventoryComponent_C"))
  (Utilities|FlowControl|Sequence
    (:then_0
      (Utilities|IsValid Instigator
        (:Is%20Valid
          (Utilities|IsValid _returnvalue
            (:Is%20Valid
              (bind _returnvalue_2 (Class|InventoryComponent|AddItem _returnvalue (Variables|Default|GetItem%20ID) (Variables|Default|GetQuantity)))
              (LocalVariables|SetRamainQuan _returnvalue_2))))))
    (:then_1
      (if (<= (LocalVariables|GetRamainQuan) 0)
        (Actor|DestroyActor)
        (else
          (Variables|Default|SetQuantity (LocalVariables|GetRamainQuan)))))))

(fn GetInteractionData
  (bind _datatable (Class|BPIPlayer|GetItemDataTable(Message) (Game|Player|GetPlayerPawn 0)))
  (Utilities|IsValid _datatable
    (:Is%20Valid
      (bind _returnvalue (Utilities|GetDataTableRow _datatable (Variables|Default|GetItem%20ID))
        (:then
          (return (.ItemName (Utilities|Struct|BreakItemData _returnvalue)) (Variables|Default|GetQuantity) (.Image (Utilities|Struct|BreakItemData _returnvalue))))
        (:RowNotFound
          _)))
    (:Is%20Not%20Valid
      _))
  (return "" 0 "/Game/Assets/Image/TD_问号.TD_问号"))