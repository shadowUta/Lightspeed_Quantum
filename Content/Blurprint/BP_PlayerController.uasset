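; Player controller that shows the mouse cursor, adds the default Enhanced Input mapping context, and creates the viewport HUD widget on BeginPlay.
; An ability update event walks the ability data array and drives the HUD's matching ability icon by index.
; For each valid ability class, it sets cooldown progress, icon and level, reading max cooldown and icon from the class defaults and remaining time and level from the data.
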(event EventBeginPlay
  (Input|AddMappingContext (PlayerController|LocalPlayerSubsystems|GetEnhancedInputLocalPlayerSubsystem) "/Game/Blurprint/Input/IMC_Default.IMC_Default" 0 "(bIgnoreAllPressedKeysUntilRelease=True,bForceImmediately=False,bNotifyUserSettings=False)")
  (bind _returnvalue (Game|ConstructObjectfromClass "/Game/Blurprint/Widget/WBP_Viweport.WBP_Viweport_C"))
  (bind _output_get (Variables|Default|SetViweport _returnvalue))
  (UserInterface|Viewport|AddtoViewport _returnvalue 0))

(event EventTick
  (params (DeltaSeconds :type Float%20%28single-precision%29)))

(event EventOnAbilityUpdate
  (params (AbilityData :type Array%20of%20Ability%20Property%20Structures))
  (for (_array_element _array_index) AbilityData
    (Utilities|IsValid (Utilities|Array|Get(acopy) (Variables|/Game/Blurprint/Widget/WBP_Viweport.WBP_Viweport_C|GetAbilityIcon (Variables|Default|GetViweport)) _array_index)
      (:Is%20Valid
        (if (Utilities|IsValidClass (.AbilityClass (Utilities|Struct|BreakAbilityProperty _array_element)))
          (Default|SetCDPercentage (Utilities|Array|Get(acopy) (Variables|/Game/Blurprint/Widget/WBP_Viweport.WBP_Viweport_C|GetAbilityIcon (Variables|Default|GetViweport)) _array_index) (.CooldownTime (Utilities|Struct|BreakAbilityProperty _array_element)) (.CooldownTime (Utilities|GetClassDefaults (.AbilityClass (Utilities|Struct|BreakAbilityProperty _array_element)))))
          (Default|SetIcon (Utilities|Array|Get(acopy) (Variables|/Game/Blurprint/Widget/WBP_Viweport.WBP_Viweport_C|GetAbilityIcon (Variables|Default|GetViweport)) _array_index) (.Image (Utilities|GetClassDefaults (.AbilityClass (Utilities|Struct|BreakAbilityProperty _array_element)))))
          (Default|SetLevel (Utilities|Array|Get(acopy) (Variables|/Game/Blurprint/Widget/WBP_Viweport.WBP_Viweport_C|GetAbilityIcon (Variables|Default|GetViweport)) _array_index) (.AbilityLevel (Utilities|Struct|BreakAbilityProperty _array_element))))))))

(fn ConstructionScript
  (Variables|Default|SetbShowMouseCursor true))