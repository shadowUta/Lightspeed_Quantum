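; Base enemy character, driven by a behavior tree and AI perception, that attacks player characters.
; BeginPlay applies move speed, passes attack range to the Blackboard and sight radius to YixiEnemyAIController, binds death, then fills two ability slots next tick.
; ExecuteAttack deals AP-based damage, while Attack calls UpgradeAbility on the ability component.
; Death stops AI logic and collision before delayed destruction; AggroSphere is sized to sight radius, but its targeting logic is disconnected.
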(event OnComponentBeginOverlap(AggroSphere)
  (params (OverlappedComponent :type Primitive%20Component%20Object%20Reference) (OtherActor :type Actor%20Object%20Reference) (OtherComp :type Primitive%20Component%20Object%20Reference) (OtherBodyIndex :type Integer) (bFromSweep :type Boolean) (SweepResult :type Hit%20Result%20Structure%20%28by%20ref%29))
  ;[0.15 0.15 0.15 0.5] 寻敌
  ;;[0.15 0.15 0.15 0.5] 玩家靠近
)

(event OnComponentEndOverlap(AggroSphere)
  (params (OverlappedComponent :type Primitive%20Component%20Object%20Reference) (OtherActor :type Actor%20Object%20Reference) (OtherComp :type Primitive%20Component%20Object%20Reference) (OtherBodyIndex :type Integer))
  ;[0.15 0.15 0.15 0.5] 寻敌
  ;;[0.15 0.15 0.15 0.5] 玩家远离
)

(event Custom|Actor_Dead
  (bind _self self)
  (bind _returnvalue (AI|GetAIController _self))
  ;[0.15 0.15 0.15 0.5] 怪物死亡
  (Utilities|FlowControl|DoOnce false
    (:Completed
      (Utilities|IsValid _returnvalue
        (:Is%20Valid
          (AI|Logic|StopLogic (Variables|/Script/AIModule.AIController|GetBrainComponent _returnvalue) ""))
        (:Is%20Not%20Valid
          _))
      (Collision|SetCollisionEnabled (Variables|Default|GetCapsuleComponent) "NoCollision")
      (Development|PrintString "怪物阵亡！")
      (Utilities|FlowControl|Delay 1.0)
      (Actor|DestroyActor))))

(event Custom|Attack
  (Default|UpgradeAbility :self (Variables|Default|GetAbilityComponent) :Level 3))

(event Collision|EventActorBeginOverlap
  (params (OtherActor :type Actor%20Object%20Reference)))

(event EventTick
  (params (DeltaSeconds :type Float%20%28single-precision%29)))

(event EventExecuteAttack
  (params (TargetActor :type Actor%20Object%20Reference))
  ;[0.15 0.15 0.15 0.5] 攻击
  (bind _asas_character (Utilities|Casting|CastToAS_Character TargetActor))
  (Default|ApplyDamage _asas_character self (Utilities|Struct|MakeUDS_DamageData (.current (Variables|Default|GetAP)) "NewEnumerator0")))

(event EventBeginPlay
  (bind _sightradius (Variables|Default|GetSightRadius))
  (bind _abilitycomponent (Variables|Default|GetAbilityComponent))
  ;[0.15 0.15 0.15 0.5] 初始化
  (Utilities|FlowControl|Sequence
    (:then_0
      ;[0.15 0.15 0.15 0.5] 初始化速度
      (Variables|/Script/Engine.CharacterMovementComponent|SetMaxWalkSpeed (Variables|Character|GetCharacterMovement) (.current (Variables|Default|GetSpeed))))
    (:then_1
      ;[0.15 0.15 0.15 0.5] 初始化攻击范围 (1) 行为树
      (AI|Components|Blackboard|SetValueasFloat (AI|GetBlackboard (Pawn|GetController)) (Utilities|Name|MakeLiteralName "AttackRange") (Variables|Default|GetAttackRange)))
    (:then_2
      ;[0.15 0.15 0.15 0.5] 初始化攻击范围 (2) AI感知组件
      (bind _asyixi_enemy_aicontroller (Utilities|Casting|CastToYixiEnemyAIController (Pawn|GetController)))
      (Class|YixiEnemyAIController|UpdateSightRadius _asyixi_enemy_aicontroller _sightradius (+ _sightradius 2e+02)))
    (:then_3
      (EventDispatchers|BindEventtoDead (EventDispatchers|CreateEvent :!event Custom|Actor_Dead)))
    (:then_4
      (Utilities|FlowControl|DelayUntilNextTick)
      (Default|ReplaceAbility _abilitycomponent 0 "(TagName=\"Ability.Enemy.text\")")
      (Default|ReplaceAbility _abilitycomponent 1 "(TagName=\"Ability.Enemy.text\")"))))

(fn ConstructionScript
  (|CallParentFunction)
  (Components|Sphere|SetSphereRadius (Variables|Default|GetAggroSphere) (Variables|Default|GetSightRadius) true))

(fn GetAttackRange
  (return (Variables|Default|GetAttackRange)))

(fn GetAttackSpeed
  (return (.current (Variables|Default|GetAttackSpeed))))