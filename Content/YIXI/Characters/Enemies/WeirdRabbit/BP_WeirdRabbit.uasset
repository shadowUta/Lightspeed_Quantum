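; BP_WeirdRabbit is an enemy character whose Attack deals area damage to players around it.
; When its state allows attacking and it is not falling, Attack clears CanAttack and starts a short timer.
; A multi-sphere trace for pawns, slightly wider than AttackRange, sends current AP as damage to Player-tagged hits through an ApplyDamage message.
; The trace draws debug shapes, and the event graph holds only disabled default events.
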(event EventBeginPlay
  (|CallParentFunction) ; 此节点被禁用，将不会被调用。\n从引脚连出引线来编译功能。
)

(event Collision|EventActorBeginOverlap
  (params (OtherActor :type Actor%20Object%20Reference))
  (|CallParentFunction OtherActor) ; 此节点被禁用，将不会被调用。\n从引脚连出引线来编译功能。
)

(event EventTick
  (params (DeltaSeconds :type Float%20%28single-precision%29))
  (|CallParentFunction DeltaSeconds) ; 此节点被禁用，将不会被调用。\n从引脚连出引线来编译功能。
)

(fn ConstructionScript
  (|CallParentFunction))

(fn Attack
  (bind _returnvalue (Transformation|GetActorLocation))
  (if (.canattack (Class|LQCharacter|GetCharacterState))
    (if (not (AI|Components|NavMovement|IsFalling (Pawn|GetMovementComponent)))
      (Class|LQCharacter|SetCanAttack false)
      (Utilities|Time|SetTimerbyEvent (EventDispatchers|CreateEvent :!event AttackCoolDown) 1.0)
      (bind _outhits (Collision|MultiSphereTraceForObjects _returnvalue _returnvalue (+ (Variables|Default|GetAttackRange) 1e+01) (Utilities|Array|MakeArray "ObjectTypeQuery3") false 0 "ForDuration" true "(R=1.000000,G=0.000000,B=0.000000,A=1.000000)" "(R=0.000000,G=1.000000,B=0.000000,A=1.000000)" 1.0))
      (for _array_element _outhits
        (if (Actor|ActorHasTag (.HitActor (Collision|BreakHitResult _array_element)) "Player")
          (Class|BPIAS|ApplyDamage(Message) (.HitActor (Collision|BreakHitResult _array_element)) self (Utilities|Struct|MakeUDS_DamageData (.current (Variables|Default|GetAP)) "NewEnumerator0")))))))