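; Base enemy Blueprint that detects the player and deals attack damage, with decisions handed to an AI controller's Blackboard.
; An aggro sphere, sized from SightRadius in the construction script, sets the Blackboard TargetActor when a Player-tagged actor enters and clears it on exit.
; ExecuteAttack applies damage to the supplied target using current AP, and GetAttackSpeed exposes the current attack speed.
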(event OnComponentBeginOverlap(AggroSphere)
  (params (OverlappedComponent :type Primitive%20Component%20Object%20Reference) (OtherActor :type Actor%20Object%20Reference) (OtherComp :type Primitive%20Component%20Object%20Reference) (OtherBodyIndex :type Integer) (bFromSweep :type Boolean) (SweepResult :type Hit%20Result%20Structure%20%28by%20ref%29))
  ;[0.15 0.15 0.15 0.5] 寻敌
  ;;[0.15 0.15 0.15 0.5] 玩家靠近
  (if (Actor|ActorHasTag OtherActor "Player")
    (AI|Components|Blackboard|SetValueasObject (AI|GetBlackboard (Pawn|GetController)) (Utilities|Name|MakeLiteralName "TargetActor") OtherActor)))

(event OnComponentEndOverlap(AggroSphere)
  (params (OverlappedComponent :type Primitive%20Component%20Object%20Reference) (OtherActor :type Actor%20Object%20Reference) (OtherComp :type Primitive%20Component%20Object%20Reference) (OtherBodyIndex :type Integer))
  (bind _returnvalue (Pawn|GetController))
  (bind _returnvalue_2 (AI|GetBlackboard _returnvalue))
  ;[0.15 0.15 0.15 0.5] 寻敌
  ;;[0.15 0.15 0.15 0.5] 玩家远离
  (if (Actor|ActorHasTag OtherActor "Player")
    (Utilities|IsValid _returnvalue_2
      (:Is%20Valid
        (AI|Components|Blackboard|ClearValue _returnvalue_2 (Utilities|Name|MakeLiteralName "TargetActor"))))))

(event EventBeginPlay)

(event Collision|EventActorBeginOverlap
  (params (OtherActor :type Actor%20Object%20Reference)))

(event EventTick
  (params (DeltaSeconds :type Float%20%28single-precision%29)))

(event EventExecuteAttack
  (params (TargetActor :type Actor%20Object%20Reference))
  (Game|Damage|ApplyDamage TargetActor (.current (Variables|Default|GetAP)) 0 self))

(fn ConstructionScript
  (|CallParentFunction)
  (Components|Sphere|SetSphereRadius (Variables|Default|GetAggroSphere) (Variables|Default|GetSightRadius) true))

(fn GetAttackSpeed
  (return (.current (Variables|Default|GetAttackSpeed))))